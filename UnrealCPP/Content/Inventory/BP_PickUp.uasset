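; BP_PickUp is a world item that the player can collect into the inventory.
; The construction script looks up its data table row, storing it as Information and setting the mesh, and BeginPlay writes the item name to the nameplate widget.
; Overlap by an UnrealCPPCharacter toggles nameplate visibility and the actor's own input binding for player 0.
; Pressing PutInInventory calls AddItem with the row's quantity and destroys the actor on success.
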(event `self.ReceiveBeginPlay`
  (bind _aswb_pick_up_nameplate (cast `/Game/Inventory/WB_PickUp_Nameplate` (`WidgetComponent.GetUserWidgetObject` (`self.NamePlate`))))
  (`TextBlock.SetText` (`/Game/Inventory/WB_PickUp_Nameplate.NameText` _aswb_pick_up_nameplate) (`KismetTextLibrary.Conv_StringToText` (`KismetStringLibrary.Concat_StrStr` "[A]" (`KismetStringLibrary.Conv_NameToString` (`.Name_2_D29DEE31406E76C2A6D9A5A09ACB53A2` (break `/Game/Inventory/ItemStructure` (`self.information`))))))))

(event `self.InteractionCollider.OnComponentBeginOverlap`
  (params (OverlappedComponent :type "PrimitiveComponent Object Reference") (OtherActor :type "Actor Object Reference") (OtherComp :type "PrimitiveComponent Object Reference") (OtherBodyIndex :type Integer) (bFromSweep :type Boolean) (SweepResult :type "HitResult Structure (by ref)"))
  (if (`KismetMathLibrary.ClassIsChildOf` (`GameplayStatics.GetObjectClass` OtherActor) "/Script/UnrealCPP.UnrealCPPCharacter")
    (`SceneComponent.SetVisibility` (`self.NamePlate`) true false)
    (`self.EnableInput` (`GameplayStatics.GetPlayerController` 0))))

(event `self.InteractionCollider.OnComponentEndOverlap`
  (params (OverlappedComponent :type "PrimitiveComponent Object Reference") (OtherActor :type "Actor Object Reference") (OtherComp :type "PrimitiveComponent Object Reference") (OtherBodyIndex :type Integer))
  (if (`KismetMathLibrary.ClassIsChildOf` (`GameplayStatics.GetObjectClass` OtherActor) "/Script/UnrealCPP.UnrealCPPCharacter")
    (`SceneComponent.SetVisibility` (`self.NamePlate`) false false)
    (`self.DisableInput` (`GameplayStatics.GetPlayerController` 0))))

(event `InputAction|PutInInventory`
  (params (Key :type "Key Structure"))
  (bind _information (`self.information`))
  (:`Pressed`
    (bind _successfullyadded (`/Game/Inventory/BPFunctionLibrary.AddItem` _information (`.Quantity_20_4E58940240153F3F417B35A1FEEEEB4D` (break `/Game/Inventory/ItemStructure` _information))))
    (if _successfullyadded
      (`self.K2_DestroyActor`))))

(fn `UserConstructionScript`
  (bind (_datatable _rowname) (break `DataTableRowHandle` (`self.item`)))
  (bind _returnvalue (`|GetDataTableRow` _datatable _rowname)
    (:`then`
      (bind _output_get (set `self.information` _returnvalue))
      (`StaticMeshComponent.SetStaticMesh` (`self.Model`) (`.Model_14_F15FD9CC44B386D9F11288AECFC51D87` (break `/Game/Inventory/ItemStructure` _output_get))))))